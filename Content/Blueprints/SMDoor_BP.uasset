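; SMDoor_BP is an interactive door that swings open when a nearby character presses Interactive while it is unlocked, then closes itself.
; Front and back trigger volumes enable input and record the approach side, which selects one of two timelines driving the mesh's yaw.
; A one-shot flag in the timeline update schedules the delayed reverse playback, while trigger overlap events stay off until a further delay restores them.
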(event `self.triggerSpaceFront.OnComponentBeginOverlap`
  (params (OverlappedComponent :type "PrimitiveComponent Object Reference") (OtherActor :type "Actor Object Reference") (OtherComp :type "PrimitiveComponent Object Reference") (OtherBodyIndex :type Integer) (bFromSweep :type Boolean) (SweepResult :type "HitResult Structure (by ref)"))
  ;[1 1 1] 判断人物来向
  (cast `Character` OtherActor)
  (`self.EnableInput` (`GameplayStatics.GetPlayerController` 0))
  (set `self.PawnfromFront` true))

(event `self.triggerSpaceFront.OnComponentEndOverlap`
  (params (OverlappedComponent :type "PrimitiveComponent Object Reference") (OtherActor :type "Actor Object Reference") (OtherComp :type "PrimitiveComponent Object Reference") (OtherBodyIndex :type Integer))
  ;[1 1 1] 判断人物来向
  (cast `Character` OtherActor)
  (`self.DisableInput` (`GameplayStatics.GetPlayerController` 0)))

(event `self.triggerSpaceBack.OnComponentBeginOverlap`
  (params (OverlappedComponent :type "PrimitiveComponent Object Reference") (OtherActor :type "Actor Object Reference") (OtherComp :type "PrimitiveComponent Object Reference") (OtherBodyIndex :type Integer) (bFromSweep :type Boolean) (SweepResult :type "HitResult Structure (by ref)"))
  ;[1 1 1] 判断人物来向
  (cast `Character` OtherActor)
  (`self.EnableInput` (`GameplayStatics.GetPlayerController` 0))
  (set `self.PawnfromFront` false))

(event `self.triggerSpaceBack.OnComponentEndOverlap`
  (params (OverlappedComponent :type "PrimitiveComponent Object Reference") (OtherActor :type "Actor Object Reference") (OtherComp :type "PrimitiveComponent Object Reference") (OtherBodyIndex :type Integer))
  ;[1 1 1] 判断人物来向
  (cast `Character` OtherActor)
  (`self.DisableInput` (`GameplayStatics.GetPlayerController` 0)))

(event `InputAction|Interactive`
  (params (Key :type "Key Structure" :default "AnyKey"))
  (bind _staticmeshcomponent (`self.StaticMeshComponent`))
  (bind _shouldclose (`self.shouldClose`))
  (:`Pressed`
    (set `self.shouldClose` true)
    (if (`self.isUnlocked`)
      (set `PrimitiveComponent.bGenerateOverlapEvents` false (`self.triggerSpaceFront`))
      (set `PrimitiveComponent.bGenerateOverlapEvents` false (`self.triggerSpaceBack`))
      (if (`self.PawnfromFront`)
        (bind (_direction _zpoint) (`Timeline|doorRotato_F` :!via `PlayFromStart` :!label _label)
          (:`Update`
            (`SceneComponent.K2_SetRelativeRotation` _staticmeshcomponent (`KismetMathLibrary.MakeRotator` 0.0 0.0 (+ (* _zpoint 100.0) 90.0)) false false)
            (if _shouldclose
              (set `self.shouldClose` false)
              (`KismetSystemLibrary.Delay` 5.0)
              (goto _label :!via `ReverseFromEnd`)
              (else
                (`KismetSystemLibrary.Delay` 6.0 :!label _label_2)
                (set `PrimitiveComponent.bGenerateOverlapEvents` true (`self.triggerSpaceFront`))
                (set `PrimitiveComponent.bGenerateOverlapEvents` true (`self.triggerSpaceBack`))))))
        (else
          (bind (_direction_2 _zpoint_2) (`Timeline|doorRotato_B` :!via `PlayFromStart` :!label _label_3)
            (:`Update`
              (`SceneComponent.K2_SetRelativeRotation` _staticmeshcomponent (`KismetMathLibrary.MakeRotator` 0.0 0.0 (+ (* _zpoint_2 100.0) 90.0)) false false)
              (if _shouldclose
                (set `self.shouldClose` false)
                (`KismetSystemLibrary.Delay` 5.0)
                (goto _label_3 :!via `ReverseFromEnd`)
                (else
                  (goto _label_2))))))))))

(fn `UserConstructionScript`)