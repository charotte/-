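; Bathroom door actor that the player opens with the Interactive input once a matching key unlocks it.
; Front and back trigger volumes enable input and record the approach side, selecting one of two timelines that drive the mesh's yaw.
; Interacting consumes the key from MyCharacter's Items, or prints a locked message without one.
; The door auto-reverses after a delay, with trigger overlap events temporarily disabled to avoid an endless-opening bug.
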(event `self.triggerSpaceFront.OnComponentBeginOverlap`
  (params (OverlappedComponent :type "PrimitiveComponent Object Reference") (OtherActor :type "Actor Object Reference") (OtherComp :type "PrimitiveComponent Object Reference") (OtherBodyIndex :type Integer) (bFromSweep :type Boolean) (SweepResult :type "HitResult Structure (by ref)"))
  ;[1 1 1] 判断人物来向
  (cast `Character` OtherActor)
  (`self.EnableInput` (`GameplayStatics.GetPlayerController` 0))
  (set `self.PawnfromFront` true))

(event `self.triggerSpaceFront.OnComponentEndOverlap`
  (params (OverlappedComponent :type "PrimitiveComponent Object Reference") (OtherActor :type "Actor Object Reference") (OtherComp :type "PrimitiveComponent Object Reference") (OtherBodyIndex :type Integer))
  ;[1 1 1] 判断人物来向
  (cast `Character` OtherActor)
  (`self.DisableInput` (`GameplayStatics.GetPlayerController` 0)))

(event `self.triggerSpaceBack.OnComponentBeginOverlap`
  (params (OverlappedComponent :type "PrimitiveComponent Object Reference") (OtherActor :type "Actor Object Reference") (OtherComp :type "PrimitiveComponent Object Reference") (OtherBodyIndex :type Integer) (bFromSweep :type Boolean) (SweepResult :type "HitResult Structure (by ref)"))
  ;[1 1 1] 判断人物来向
  (cast `Character` OtherActor)
  (`self.EnableInput` (`GameplayStatics.GetPlayerController` 0))
  (set `self.PawnfromFront` false))

(event `self.triggerSpaceBack.OnComponentEndOverlap`
  (params (OverlappedComponent :type "PrimitiveComponent Object Reference") (OtherActor :type "Actor Object Reference") (OtherComp :type "PrimitiveComponent Object Reference") (OtherBodyIndex :type Integer))
  ;[1 1 1] 判断人物来向
  (cast `Character` OtherActor)
  (`self.DisableInput` (`GameplayStatics.GetPlayerController` 0)))

(event `InputAction|Interactive`
  (params (Key :type "Key Structure" :default "AnyKey"))
  (bind _staticmeshcomponent (`self.StaticMeshComponent`))
  (bind _shouldclose (`self.shouldClose`))
  (:`Pressed`
    (`self.CheckKeyExists`)
    (set `self.shouldClose` true)
    ;[1 1 1] 通过关闭重叠事件来避免无限开门BUG
    (if (`self.isUnlocked`)
      (set `PrimitiveComponent.bGenerateOverlapEvents` false (`self.triggerSpaceBack`))
      (set `PrimitiveComponent.bGenerateOverlapEvents` false (`self.triggerSpaceFront`))
      (if (`self.PawnfromFront`)
        (bind (_direction _zpoint) (`Timeline|doorRotato_F` :!via `PlayFromStart` :!label _label)
          (:`Update`
            (`SceneComponent.K2_SetRelativeRotation` _staticmeshcomponent (`KismetMathLibrary.MakeRotator` 0.0 0.0 (+ (* _zpoint 100.0) 0.0)) false false)
            (if _shouldclose
              (set `self.shouldClose` false)
              (`KismetSystemLibrary.Delay` 5.0)
              (goto _label :!via `ReverseFromEnd`)
              (else
                (`KismetSystemLibrary.Delay` 6.0 :!label _label_2)
                (set `PrimitiveComponent.bGenerateOverlapEvents` true (`self.triggerSpaceBack`))
                (set `PrimitiveComponent.bGenerateOverlapEvents` true (`self.triggerSpaceFront`))))))
        (else
          (bind (_direction_2 _zpoint_2) (`Timeline|doorRotato_B` :!via `PlayFromStart` :!label _label_3)
            (:`Update`
              (`SceneComponent.K2_SetRelativeRotation` _staticmeshcomponent (`KismetMathLibrary.MakeRotator` 0.0 0.0 (+ (* _zpoint_2 100.0) 0.0)) false false)
              (if _shouldclose
                (set `self.shouldClose` false)
                (`KismetSystemLibrary.Delay` 5.0)
                (goto _label_3 :!via `ReverseFromEnd`)
                (else
                  (goto _label_2)))))))
      (else
        (`KismetSystemLibrary.PrintText` "浴室门锁住了，打不开")))))

(event `CheckKeyExists`
  (bind _asmy_character (cast `/Game/ThirdPersonBP/Blueprints/MyCharacter` (`GameplayStatics.GetPlayerCharacter` 0)))
  (bind _items (`/Game/ThirdPersonBP/Blueprints/MyCharacter.Items` _asmy_character))
  (for (_array_element _array_index) _items
    (if (== (break `/Game/Blueprints/Item` _array_element) (`.ItemID_2_CDE609C04D6AF7F448EF3F9D996A5054` (break `/Game/Blueprints/Item` (`self.Bathkey`))))
      (`KismetArrayLibrary.Array_Remove` _items _array_index)
      (set `self.isUnlocked` true)
      (`KismetSystemLibrary.PrintText` "浴室门打开了")
      (`KismetSystemLibrary.Delay` 1.0)
      (break))))

(fn `UserConstructionScript`)