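; BathroomKey is a pickup actor that the player collects with the Interactive input while standing near it.
; Its TriggerSpace overlap enables and disables the actor's input when MyCharacter enters or leaves.
; Pressing Interactive prints the item description, passes ItemInfo to the controlled MyCharacter through GetItem, then destroys the actor.
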(event `self.triggerSpace.OnComponentBeginOverlap`
  (params (OverlappedComponent :type "PrimitiveComponent Object Reference") (OtherActor :type "Actor Object Reference") (OtherComp :type "PrimitiveComponent Object Reference") (OtherBodyIndex :type Integer) (bFromSweep :type Boolean) (SweepResult :type "HitResult Structure (by ref)"))
  (cast `/Game/ThirdPersonBP/Blueprints/MyCharacter` OtherActor)
  (`self.EnableInput` (`GameplayStatics.GetPlayerController` 0)))

(event `self.triggerSpace.OnComponentEndOverlap`
  (params (OverlappedComponent :type "PrimitiveComponent Object Reference") (OtherActor :type "Actor Object Reference") (OtherComp :type "PrimitiveComponent Object Reference") (OtherBodyIndex :type Integer))
  (cast `/Game/ThirdPersonBP/Blueprints/MyCharacter` OtherActor)
  (`self.DisableInput` (`GameplayStatics.GetPlayerController` 0)))

(event `InputAction|Interactive`
  (params (Key :type "Key Structure" :default "AnyKey"))
  (bind _iteminfo (`self.ItemInfo`))
  (:`Pressed`
    (`KismetSystemLibrary.PrintText` (`.ItemDescription_12_78442B2A4DF1F8010D944794BDDBC76E` (break `/Game/Blueprints/Item` _iteminfo)))
    (bind _asmy_character (cast `/Game/ThirdPersonBP/Blueprints/MyCharacter` (`Controller.K2_GetPawn` (`GameplayStatics.GetPlayerController` 0))))
    (`/Game/ThirdPersonBP/Blueprints/MyCharacter.GetItem` _asmy_character _iteminfo)
    (`self.K2_DestroyActor`)))

(fn `UserConstructionScript`)